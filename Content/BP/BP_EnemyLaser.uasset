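; Enemy laser Blueprint that fires a timed beam segment, drawn with a beam particle, along the particle's forward axis.
; Emit resets and activates the beam; each Tick extends the front at BeamSpeed, and after the emit time the tail follows until the segment collapses and deactivates.
; A debug-drawn Visibility trace between tail and front sets the beam endpoints and shortens it at obstacles, with distances clamped to BeamLenMax.
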(event EventTick
  (params (DeltaSeconds :type Float%20%28single-precision%29))
  (bind _beamparticle (Variables|Default|GetBeamParticle))
  (bind _beamspeed (Variables|Default|GetBeamSpeed))
  (bind _beamparticle_2 (Variables|Default|GetBeamParticle))
  (bind _returnvalue (Transformation|GetWorldLocation _beamparticle_2))
  (bind _returnvalue_2 (Transformation|GetWorldRotation _beamparticle_2))
  (bind _returnvalue_3 (* DeltaSeconds _beamspeed))
  (bind _returnvalue_4 (Math|Vector|GetForwardVector _returnvalue_2))
  (if (Components|Activation|IsActive (Variables|Default|GetBeamParticle))
    (Utilities|FlowControl|Sequence
      (:then_0
        ;[1 1 1] 時間を計測
        (Variables|Default|SetEmitTimer (+ (Variables|Default|GetEmitTimer) DeltaSeconds)))
      (:then_1
        (if (Variables|Default|GetEmitStop)
          (CallFunction|SetEmitEndDistance (+ (Variables|Default|GetEmitEndDistance) _returnvalue_3))
          (CallFunction|SetEmitStartDistance (+ (Variables|Default|GetEmitStartDistance) _returnvalue_3))
          (else
            (Variables|Default|SetEmitStop (>= (Variables|Default|GetEmitTimer) (Variables|Default|GetEmitStopTime)))
            (CallFunction|SetEmitEndDistance (+ (Variables|Default|GetEmitEndDistance) _returnvalue_3)))))
      (:then_2
        (if (and (Variables|Default|GetEmitStop) (< (Math|Float|Absolute(Float) (- (Variables|Default|GetEmitStartDistance) (Variables|Default|GetEmitEndDistance))) 1.0))
          (Components|Activation|Deactivate (Variables|Default|GetBeamParticle))))
      (:then_3
        (bind _outhit (Collision|LineTraceByChannel (+ _returnvalue (* _returnvalue_4 (Variables|Default|GetEmitStartDistance))) (+ _returnvalue (* _returnvalue_4 (Variables|Default|GetEmitEndDistance))) "TraceTypeQuery1" false 0 "ForDuration"))
        (Class|ParticleSystemComponent|SetBeamSourcePoint _beamparticle 0 (.TraceStart (Collision|BreakHitResult _outhit)))
        (if (.bBlockingHit (Collision|BreakHitResult _outhit))
          ;[1 1 1] ビームが障害物に当たったら
          (Class|ParticleSystemComponent|SetBeamTargetPoint _beamparticle 0 (.Location (Collision|BreakHitResult _outhit)))
          (CallFunction|SetEmitEndDistance (Math|Vector|VectorLength (- (.Location (Collision|BreakHitResult _outhit)) (Transformation|GetWorldLocation _beamparticle))))
          (else
            ;[1 1 1] 障害物に当たらなかったら
            (Class|ParticleSystemComponent|SetBeamTargetPoint _beamparticle 0 (.TraceEnd (Collision|BreakHitResult _outhit)))))))))

(fn ConstructionScript)

(fn Emit
  (params (EmitTime :type Float%20%28double-precision%29))
  (Variables|Default|SetEmitStopTime EmitTime)
  (Variables|Default|SetEmitTimer 0.0)
  (Variables|Default|SetEmitStartDistance 0.0)
  (Variables|Default|SetEmitEndDistance 0.0)
  (Variables|Default|SetEmitStop false)
  (Components|Activation|Activate (Variables|Default|GetBeamParticle) false))

(fn SetEmitStartDistance
  (params (EmitStartDistance :type Float%20%28double-precision%29))
  (Variables|Default|SetEmitStartDistance (Math|Float|Min(Float) EmitStartDistance (Variables|Default|GetEmitEndDistance))))

(fn SetEmitEndDistance
  (params (Distance :type Float%20%28double-precision%29))
  (Variables|Default|SetEmitEndDistance (Math|Float|Min(Float) Distance (Variables|Default|GetBeamLenMax)))
  (CallFunction|SetEmitStartDistance (Variables|Default|GetEmitStartDistance)))