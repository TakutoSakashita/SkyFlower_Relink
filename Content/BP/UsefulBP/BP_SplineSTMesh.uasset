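; Utility actor that scatters copies of a static mesh along an editable spline.
; The Construction Script adds MeshCount instances to an InstancedStaticMesh component at equal distance intervals, using the spline's local-space location and rotation at each point.
; Spacing is spline length divided by MeshCount, so the first instance sits at the start and none is placed at the end distance.
; The event graph holds only disabled default events.
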(event EventBeginPlay)

(event Collision|EventActorBeginOverlap
  (params (OtherActor :type Actor%20Object%20Reference)))

(event EventTick
  (params (DeltaSeconds :type Float%20%28single-precision%29)))

(fn ConstructionScript
  (bind _spline (Variables|Default|GetSpline))
  (for _index (range 0 (- (Variables|Default|GetMeshCount) 1))
    (Components|InstancedStaticMesh|AddInstance (Variables|Default|GetInstancedStaticMesh) (Math|Transform|MakeTransform (Spline|GetLocationatDistanceAlongSpline _spline (* (/ (Math|Conversions|ToFloat(Integer) _index) (Math|Conversions|ToFloat(Integer) (Variables|Default|GetMeshCount))) (Spline|GetSplineLength (Variables|Default|GetSpline))) "Local") (Spline|GetRotationatDistanceAlongSpline _spline (* (/ (Math|Conversions|ToFloat(Integer) _index) (Math|Conversions|ToFloat(Integer) (Variables|Default|GetMeshCount))) (Spline|GetSplineLength (Variables|Default|GetSpline))) "Local") "1.000000,1.000000,1.000000") false)))