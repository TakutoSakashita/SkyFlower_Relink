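; Utility Blueprint that lays out rows of repeated static meshes in a straight line, built in the Construction Script.
; Each LinearDataList entry gets its own Instanced Static Mesh component with that entry's mesh, stored in InstancedSTMeshList.
; A second pass adds MeshCount instances per component along local Y at that entry's Distance spacing, with every row starting at the component origin.
; It has no active runtime logic.
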(event EventBeginPlay)

(event Collision|EventActorBeginOverlap
  (params (OtherActor :type Actor%20Object%20Reference)))

(event EventTick
  (params (DeltaSeconds :type Float%20%28single-precision%29)))

(fn ConstructionScript
  (for _array_element (Variables|Default|GetLinearDataList)
    (bind _returnvalue (AddComponent|AddInstancedStaticMeshComponent false))
    (Components|StaticMesh|SetStaticMesh _returnvalue (.staticmesh _array_element))
    (Utilities|Array|Add (Variables|Default|GetInstancedSTMeshList) _returnvalue))
  (for (_array_element_2 _array_index) (Variables|Default|GetInstancedSTMeshList)
    (for _index (range 0 (- (.meshcount (Utilities|Array|Get(acopy) (Variables|Default|GetLinearDataList) _array_index)) 1))
      (Components|InstancedStaticMesh|AddInstance _array_element_2 (Math|Transform|MakeTransform (Math|Vector|MakeVector 0.0 (* _index (.distance (Utilities|Array|Get(acopy) (Variables|Default|GetLinearDataList) _array_index))) 0.0)) false))))