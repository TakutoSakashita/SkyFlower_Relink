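; BP_Door is a level-exit door that stays locked until the game mode reports that an object has been destroyed.
; On BeginPlay it binds to BP_SFA_GameMode's OnObjectDestroyed dispatcher, which calls OnObjectDestroy to set the OnDestroy flag.
; When the player overlaps its Box, it opens Map_midBoss_anim if the flag is set, and otherwise prints a "cannot enter" message.
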(event OnComponentBeginOverlap(Box)
  (params (OverlappedComponent :type Primitive%20Component%20Object%20Reference) (OtherActor :type Actor%20Object%20Reference) (OtherComp :type Primitive%20Component%20Object%20Reference) (OtherBodyIndex :type Integer) (bFromSweep :type Boolean) (SweepResult :type Hit%20Result%20Structure%20%28by%20ref%29))
  (Utilities|Casting|CastToBP_SFA_Player_modelTest OtherActor)
  (if (Variables|Default|GetOnDestroy)
    (Game|OpenLevel(byObjectReference) "/Game/Maps/Map_midBoss_anim.Map_midBoss_anim")
    (else
      (Development|PrintString "入れない"))))

(event Custom|カスタムイベント
  (CallFunction|OnObjectDestroy))

(event EventBeginPlay
  (bind _asbp_sfa_game_mode (Utilities|Casting|CastToBP_SFA_GameMode (Game|GetGameMode)))
  (EventDispatchers|BindEventtoOnObjectDestroyed _asbp_sfa_game_mode (delegate Custom|カスタムイベント)))

(fn ConstructionScript)

(fn OnObjectDestroy
  (Variables|Default|SetOnDestroy true))