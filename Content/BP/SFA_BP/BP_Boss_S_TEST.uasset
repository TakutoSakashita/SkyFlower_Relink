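; BP_Boss_S_TEST is a test boss actor that moves upward once the player enters its trigger.
; Trigger overlap casts the other actor to SFA_Player, fires MovingUp, then sets HasMovingUp so later overlaps are ignored.
; MovingUp plays a timeline that, on each update, adds ZSpeed scaled by the curve value to the actor's Z location, without sweep or frame-time scaling.
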(event OnComponentBeginOverlap(Trigger)
  (params (OverlappedComponent :type Primitive%20Component%20Object%20Reference) (OtherActor :type Actor%20Object%20Reference) (OtherComp :type Primitive%20Component%20Object%20Reference) (OtherBodyIndex :type Integer) (bFromSweep :type Boolean) (SweepResult :type Hit%20Result%20Structure%20%28by%20ref%29))
  (if (not (Variables|Default|GetbHasMovingUp))
    (Utilities|Casting|CastToSFA_Player OtherActor)
    (CallFunction|MovingUp)
    (Variables|Default|SetbHasMovingUp true)))

(event Custom|MovingUp
  (bind _timeline (Timeline|Timeline Play)
    (:Update
      (Transformation|SetActorLocation (+ (Transformation|GetActorLocation) (Math|Vector|MakeVector 0.0 0.0 (* (Variables|Default|GetZ_speed) _timeline))) false false))))

(event EventBeginPlay)

(event Collision|EventActorBeginOverlap
  (params (OtherActor :type Actor%20Object%20Reference)))

(event EventTick
  (params (DeltaSeconds :type Float%20%28single-precision%29)))

(fn ConstructionScript)