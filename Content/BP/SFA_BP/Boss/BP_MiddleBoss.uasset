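; BP_MiddleBoss is a mid-boss that starts its StateTree logic when the player overlaps its activation trigger.
; It exposes action events: a timeline-driven rise that flags completion, and three attacks.
; Bubble spawns a BP_Fireball at the boss, slash plays a montage with both arm Niagara effects active until completion, and diving is delegated to BP_DivingManager actors through OnDiving.
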(event OnComponentBeginOverlap(TriggerActivate)
  (params (OverlappedComponent :type Primitive%20Component%20Object%20Reference) (OtherActor :type Actor%20Object%20Reference) (OtherComp :type Primitive%20Component%20Object%20Reference) (OtherBodyIndex :type Integer) (bFromSweep :type Boolean) (SweepResult :type Hit%20Result%20Structure%20%28by%20ref%29))
  ;[1 1 1] Activate trigger
  (Utilities|Casting|CastToSFA_Player OtherActor)
  (Variables|StateTree|SetbIsBossActivated true)
  (Development|PrintString "BossActivate" true false "(R=0.000000,G=1.000000,B=0.698892,A=1.000000)" 5.0)
  (AI|Logic|StartLogic (Variables|Default|GetStateTree)))

(event Custom|MovingUp
  ;[1 1 1] Moving up
  (Variables|StateTree|SetbIsMovingUpFinished false)
  (bind _timeline (Timeline|Timeline Play)
    (:Update
      (Transformation|SetActorLocation (+ (Transformation|GetActorLocation) (Math|Vector|MakeVector 0.0 0.0 (* (Variables|Default|GetZ_speed) _timeline))) false false))
    (:Finished
      (Variables|StateTree|SetbIsMovingUpFinished true))))

(event Custom|BubbleAttack
  ;[1 1 1] Bubble attack
  (Game|SpawnActorfromClass "/Game/Effects/FIre/BP_Fireball.BP_Fireball_C" (Math|Transform|MakeTransform (Transformation|GetActorLocation) (Transformation|GetActorRotation)) "AlwaysSpawn" "MultiplyWithRoot" 0 0))

(event Custom|SlashAttack
  ;[0 1 0] Comment
  (Components|Activation|SetActive (Variables|Default|GetNiagara_arm_right) true false)
  (Components|Activation|SetActive (Variables|Default|GetNiagara_arm_left) true false)
  (Animation|Montage|PlayMontage (Variables|Default|GetSkeletalMesh) "/Game/Boss_Middle/Animations/slash/AM_midBoss_slash.AM_midBoss_slash"
    (:OnCompleted
      (Components|Activation|SetActive (Variables|Default|GetNiagara_arm_right) false false)
      (Components|Activation|SetActive (Variables|Default|GetNiagara_arm_left) false false))))

(event Custom|DivingAttack
  ;[1 1 1] Diving attack
  (bind _outactors (Actor|GetAllActorsOfClass "/Game/Effects/Diving/BP_DivingManager.BP_DivingManager_C"))
  (Default|OnDiving _outactors))

(event Collision|EventActorBeginOverlap
  (params (OtherActor :type Actor%20Object%20Reference)))

(event EventTick
  (params (DeltaSeconds :type Float%20%28single-precision%29)))

(fn ConstructionScript)