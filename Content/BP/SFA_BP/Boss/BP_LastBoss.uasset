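; Last boss actor that starts its StateTree logic when the player overlaps its activation trigger.
; FiveLaser spawns and launches BP_Laser shots in a fan of directions around the player, built by GetFiveDirection through vector rotation.
; RotationLaser sets a flag that makes Tick turn the boss and spawn a forward bullet every frame until a short delay clears it.
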(event OnComponentBeginOverlap(TriggerActivate)
  (params (OverlappedComponent :type Primitive%20Component%20Object%20Reference) (OtherActor :type Actor%20Object%20Reference) (OtherComp :type Primitive%20Component%20Object%20Reference) (OtherBodyIndex :type Integer) (bFromSweep :type Boolean) (SweepResult :type Hit%20Result%20Structure%20%28by%20ref%29))
  ;[1 1 1] Comment
  (Utilities|Casting|CastToSFA_Player OtherActor)
  (Variables|StateTree|SetbIsBossActivated true)
  (Development|PrintString "BossActivate" true false "(R=0.000000,G=1.000000,B=0.698892,A=1.000000)" 5.0)
  (AI|Logic|StartLogic (Variables|Default|GetStateTree)))

(event Custom|FiveLaser
  (bind _returnvalue (Transformation|GetActorLocation))
  ;[1 1 1] ＦｉｖｅＬａｓｅｒ
  (bind _outdirectionlist (CallFunction|GetFiveDirection (- (Transformation|GetActorLocation (Game|Player|GetPlayerPawn 0)) (Transformation|GetActorLocation)) 1e+01))
  (for _array_element _outdirectionlist
    (bind _returnvalue_2 (Game|SpawnActorfromClass "/Game/BP/BP_Laser.BP_Laser_C" (Math|Transform|MakeTransform _returnvalue (Math|Rotator|FindLookatRotation _returnvalue (+ _array_element _returnvalue)) "1.000000,1.000000,1.000000") "Undefined" "MultiplyWithRoot" 0 0))
    (Default|LaunchLaser _returnvalue_2 (Transformation|GetActorLocation _returnvalue_2))))

(event Custom|RotationLaser
  (Variables|Default|SetbIsRotate true))

(event EventTick
  (params (DeltaSeconds :type Float%20%28single-precision%29))
  (if (Variables|Default|GetbIsRotate)
    (Transformation|SetActorRotation (Math|Conversions|RotationFromXVector (Math|Vector|RotateVector (Transformation|GetActorForwardVector) "0.000000,10.000000,0.000000")))
    (bind _returnvalue (Game|SpawnActorfromClass "/Game/BP/Bullet/BP_ForwardBullet.BP_ForwardBullet_C" (Transformation|GetActorTransform) "Undefined" "MultiplyWithRoot" 0 0))
    (Utilities|FlowControl|Delay 1.0)
    (Variables|Default|SetbIsRotate false)))

(fn ConstructionScript)

(fn GetFiveDirection
  (params (InDestinagionLocation :type Vector) (InAngle :type Float%20%28double-precision%29))
  (bind _directionlist (LocalVariables|GetDirectionList))
  ;[1 1 1] 初期化
  (LocalVariables|SetRadian InAngle)
  (Utilities|Array|Add (LocalVariables|GetDirectionList) InDestinagionLocation)
  ;[1 1 1] 入力された角度分右に基準のベクトルを回転
  (for _index (range 1 2)
    (LocalVariables|SetRadian (* (LocalVariables|GetRadian) _index))
    (Utilities|Array|Insert (LocalVariables|GetDirectionList) (Math|Vector|RotateVector (Utilities|Array|Get(acopy) _directionlist (Utilities|Array|LastIndex _directionlist)) (Math|Rotator|MakeRotator 0.0 0.0 (LocalVariables|GetRadian)))))
  (LocalVariables|SetRadian InAngle)
  ;[1 1 1] 入力された角度分左にベクトルを回転させる
  (for _index_2 (range 1 2)
    (LocalVariables|SetRadian (* (LocalVariables|GetRadian) _index_2))
    (Utilities|Array|Add (LocalVariables|GetDirectionList) (Math|Vector|RotateVector (Utilities|Array|Get(acopy) (LocalVariables|GetDirectionList) 2) (Math|Rotator|MakeRotator 0.0 0.0 (* (LocalVariables|GetRadian) -1.0)))))
  (return (LocalVariables|GetDirectionList)))