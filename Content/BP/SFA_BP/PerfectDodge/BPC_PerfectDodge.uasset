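; Player component that plays perfect dodge feedback when ApplyPerfectDodge is called while IsPerfectDodge is set.
; It clears the flag, turns on the player's dodge effect and drops global time dilation for a brief slow motion.
; A short Delay, stretched to about a real second by the dilation, then restores normal time and hides the effect.
; Debug text, sphere and arrow mark the hit point and normal.
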(event Custom|ApplyPerfectDodge
  (params (HitResult :type Hit%20Result%20Structure) (Instigator :type Actor%20Object%20Reference))
  (bind (_bblockinghit _binitialoverlap _time _distance _location _impactpoint _normal _impactnormal) (Collision|BreakHitResult HitResult))
  (if (Variables|Default|GetIsPerfectDodge)
    (Utilities|FlowControl|Sequence
      (:then_0
        (Development|PrintString "PERFECT DODGE" true true "(R=1.000000,G=0.036018,B=0.000000,A=1.000000)")
        (bind _playerref (Variables|Default|GetPlayerRef)
          (:then
            (Default|ShowPerfectDodgeEffect _playerref true)
            (Variables|Default|SetIsPerfectDodge false)
            (Utilities|Time|SetGlobalTimeDilation 0.05)
            (Rendering|Debug|DrawDebugSphere _impactpoint 1e+02 12 "(R=0.000000,G=0.723686,B=1.000000,A=1.000000)" 5.0 1e+01)
            ;[1 1 1] Comment
            (Utilities|FlowControl|Delay 0.05)
            (Utilities|Time|SetGlobalTimeDilation 1.0)
            (Default|ShowPerfectDodgeEffect (Variables|Default|GetPlayerRef) false))
          (:else)))
      (:then_1
        (Rendering|Debug|DrawDebugArrow _impactpoint (+ _impactpoint (* _impactnormal 1e+02)) 5e+01 "(R=0.000000,G=0.135954,B=1.000000,A=1.000000)" 3.0 1e+01)))))

(event EventBeginPlay
  (bind _asbp_sfa_player_model_test (Utilities|Casting|CastToBP_SFA_Player_modelTest (Components|GetOwner)))
  (Variables|Default|SetPlayerRef _asbp_sfa_player_model_test))

(event EventTick
  (params (DeltaSeconds :type Float%20%28single-precision%29)))