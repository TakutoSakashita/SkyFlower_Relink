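; Test player character Blueprint for SFA, layering prototype attack, gliding and effect hooks onto the player.
; Attack input activates a GAS ability by tag, InitWeapon caches the child-actor weapon, and Tick pitches the capsule while moving in Float without boosting.
; Events toggle dodge Niagara, print damage and show a test game-clear widget on death; a debug key toggles the camera's boost Niagara.
; Disconnected leftovers cover fly speed, aim and movement-mode tests.
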(event Custom|ShowPerfectDodgeEffect
  (params (IsVisible :type Boolean))
  ;[1 1 1] TEST Dodge
  (Rendering|SetVisibility (Variables|Default|GetNiagara_Dodge) IsVisible false))

(event EventBeginPlay
  (bind _asbp_sfa_player_controller (Utilities|Casting|CastToBP_SFA_PlayerController (Game|GetPlayerController 0)))
  (bind _asbp_sfa_camera_test (Utilities|Casting|CastToBP_SFA_Camera_TEST (Class|SFAPlayerController|GetCamera _asbp_sfa_player_controller)))
  (Variables|Default|SetAs%20BP%20SFA%20Camera%20TEST _asbp_sfa_camera_test))

(event EventTakeDamageBP
  (params (Aggresor :type Actor%20Object%20Reference) (Damage :type Float%20%28double-precision%29))
  ;[1 1 1] BP Damege Interface
  (Development|PrintString (Utilities|String|ToString(Float) Damage) true true "(R=1.000000,G=0.000000,B=0.061523,A=1.000000)"))

(event EventInitWeapon
  ;[1 1 1] Weapon
  (bind _asbp_sfa_weapon (Utilities|Casting|CastToBP_SFA_Weapon (Variables|/Script/Engine.ChildActorComponent|GetChildActor (Variables|Default|GetChildActor))))
  (Variables|Default|SetWeapon _asbp_sfa_weapon))

(event EventDie
  ;[1 1 1] Die
  (Development|PrintString "BP_SFA_PLAYER : DIE")
  (bind _returnvalue (UserInterface|CreateWidget "/Game/BP/UI/WBP_GameClearTEST.WBP_GameClearTEST_C"))
  (UserInterface|Viewport|AddtoViewport _returnvalue 0))

(event EventTick
  (params (DeltaSeconds :type Float%20%28single-precision%29))
  (bind _returnvalue (Transformation|GetActorRotation))
  ;[1 1 1] TEST gliding
  (if (Utilities|Enum|Equal(Enum) (Variables|/Script/Asterisk.SFA_InputHandlerComponent|GetMoveState (Variables|Default|GetInputHandler)) "Float")
    (if (> (Math|Vector|VectorLengthXY (Variables|/Script/Engine.MovementComponent|GetVelocity (Variables|Default|GetPlayerMovement))) 0.0)
      (if (not (Variables|/Script/Asterisk.SFA_PlayerStateMachine|GetbIsBoosting (Variables|Default|GetPlayerStateMachine)))
        (Transformation|SetRelativeRotation (Variables|Default|GetCapsuleComponent) (Math|Rotator|MakeRotator 0.0 -5e+01 (.yaw _returnvalue)) false false))
      (else
        (Transformation|SetRelativeRotation (Variables|Default|GetCapsuleComponent) (Math|Rotator|MakeRotator 0.0 0.0 (.yaw _returnvalue)) false false)))))

(event Input|KeyboardEvents|DebugKeyF12
  (params (Key :type Key%20Structure :default "None") (ActionValue :type Input%20Action%20Value%20Structure))
  ;[0 1 0] Comment
)

(event Input|KeyboardEvents|DebugKeyZ
  (params (Key :type Key%20Structure :default "None") (ActionValue :type Input%20Action%20Value%20Structure))
  ;[0.01 1 0] TEST Boost
)

(event Input|KeyboardEvents|DebugKeyQ
  (params (Key :type Key%20Structure :default "None") (ActionValue :type Input%20Action%20Value%20Structure))
  ;[0 1 0] TEST Boost Niagara Effect
  (:Pressed
    (bind _as_bp_sfa_camera_test (Variables|Default|GetAs%20BP%20SFA%20Camera%20TEST)
      (:then
        (Rendering|SetVisibility (Variables|/Game/BP/SFA_BP/Camera/BP_SFA_Camera_TEST.BP_SFA_Camera_TEST_C|GetNiagara_Boost _as_bp_sfa_camera_test) true false))
      (:else)))
  (:Released
    (bind _as_bp_sfa_camera_test_2 (Variables|Default|GetAs%20BP%20SFA%20Camera%20TEST)
      (:then
        (Rendering|SetVisibility (Variables|/Game/BP/SFA_BP/Camera/BP_SFA_Camera_TEST.BP_SFA_Camera_TEST_C|GetNiagara_Boost _as_bp_sfa_camera_test_2) false false))
      (:else))))

(event Input|GamepadEvents|GamepadFaceButtonLeft
  (params (Key :type Key%20Structure :default "None"))
  ;[1 1 1] Attack
  (:Pressed
    (Abilities|TryActivateAbilitiesbyTag (Variables|Default|GetAbilitySystem) (GameplayTags|MakeGameplayTagContainerfromTag "(TagName=\"Ability.Action.Attack\")") true)))

(event Input|MouseEvents|LeftMouseButton
  (params (Key :type Key%20Structure :default "None"))
  ;[1 1 1] Attack
  (:Pressed
    (Abilities|TryActivateAbilitiesbyTag (Variables|Default|GetAbilitySystem) (GameplayTags|MakeGameplayTagContainerfromTag "(TagName=\"Ability.Action.Attack\")") true)))

(fn ConstructionScript)