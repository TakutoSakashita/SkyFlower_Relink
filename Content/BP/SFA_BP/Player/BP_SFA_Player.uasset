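; Player Blueprint for SFA that handles attack input and weapon setup through the Gameplay Ability System and a child actor.
; Left mouse press asks the AbilitySystem to activate abilities tagged Ability.Action.Attack.
; InitWeapon casts the ChildActor's actor to BP_SFA_Weapon and caches it as Weapon.
; Leftover camera aim and flying/walking movement-mode logic is disconnected and never runs.
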(event EventBeginPlay)

(event Collision|EventActorBeginOverlap
  (params (OtherActor :type Actor%20Object%20Reference)))

(event EventTick
  (params (DeltaSeconds :type Float%20%28single-precision%29)))

(event EventInitWeapon
  ;[1 1 1] コメント
  (bind _asbp_sfa_weapon (Utilities|Casting|CastToBP_SFA_Weapon (Variables|/Script/Engine.ChildActorComponent|GetChildActor (Variables|Default|GetChildActor))))
  (Variables|Default|SetWeapon _asbp_sfa_weapon))

(event Input|KeyboardEvents|DebugKeyF12
  (params (Key :type Key%20Structure :default "None") (ActionValue :type Input%20Action%20Value%20Structure))
  ;[1 1 1] Comment
)

(event Input|MouseEvents|LeftMouseButton
  (params (Key :type Key%20Structure :default "None"))
  ;[1 1 1] Comment
  (:Pressed
    (Abilities|TryActivateAbilitiesbyTag (Variables|Default|GetAbilitySystem) (GameplayTags|MakeGameplayTagContainerfromTag "(TagName=\"Ability.Action.Attack\")") true)))

(fn ConstructionScript)