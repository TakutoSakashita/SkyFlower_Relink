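; Player gameplay ability for the first combo attack, which commits and plays the Combo1 montage.
; Montage notify windows open the follow-up: Input toggles the Ability.Ready.Combo2 tag and Branch toggles Ability.Begin.Combo2.
; The ability ends on blend out or interruption, and its end handler clears only the Begin tag.
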(event Ability|EventActivateAbility
  (Ability|CommitAbility)
  (bind _notifyname (Animation|Montage|PlayMontage (Class|GameplayAbility|GetOwningComponentfromActorInfo) "/Game/BP/SFA_BP/Player/Anim/AM_P_Combo1.AM_P_Combo1")
    (:OnBlendOut
      (Ability|EndAbility :!label _label))
    (:OnInterrupted
      (goto _label))
    (:OnNotifyBegin
      (switch name _notifyname
        (:Combo%201.Input
          (Class|SFABlogComboGameplayAbility|AddGameplayTags "(GameplayTags=((TagName=\"Ability.Ready.Combo2\")))"))
        (:Combo%201.Branch
          (Class|SFABlogComboGameplayAbility|AddGameplayTags "(GameplayTags=((TagName=\"Ability.Begin.Combo2\")))"))))
    (:OnNotifyEnd
      (switch name _notifyname
        (:Combo%201.Input
          (Class|SFABlogComboGameplayAbility|RemoveGameplayTags "(GameplayTags=((TagName=\"Ability.Ready.Combo2\")))"))
        (:Combo%201.Branch
          (Class|SFABlogComboGameplayAbility|RemoveGameplayTags "(GameplayTags=((TagName=\"Ability.Begin.Combo2\")))"))))))

(event Ability|EventOnEndAbility
  (params (bWasCancelled :type Boolean))
  (Class|SFABlogComboGameplayAbility|RemoveGameplayTags "(GameplayTags=((TagName=\"Ability.Begin.Combo2\"),(TagName=\"Ability.Ready.Combo2\")))"))