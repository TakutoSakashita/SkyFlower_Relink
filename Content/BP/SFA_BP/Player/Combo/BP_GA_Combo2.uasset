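; Gameplay ability for the second step of the player's melee or attack combo chain.
; On activation it commits, waits for the Ability.Begin.Combo2 tag, then plays the Combo2 montage.
; Input and Branch montage notify windows add and remove the Ready and Begin tags for Combo3, opening the link to the next step.
; The ability ends on blend out or interruption, clearing Ability.Begin.Combo3.
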(event Ability|EventActivateAbility
  (Ability|CommitAbility)
  (Ability|Tasks|WaitGameplayTagAdd "(TagName=\"Ability.Begin.Combo2\")" 0
    (:Added
      (bind _notifyname (Animation|Montage|PlayMontage (Class|GameplayAbility|GetOwningComponentfromActorInfo) "/Game/BP/SFA_BP/Player/Anim/AM_P_Combo2.AM_P_Combo2")
        (:OnBlendOut
          (Ability|EndAbility :!label _label))
        (:OnInterrupted
          (goto _label))
        (:OnNotifyBegin
          (switch name _notifyname
            (:Combo2.Input
              (Class|SFABlogComboGameplayAbility|AddGameplayTags "(GameplayTags=((TagName=\"Ability.Ready.Combo3\")))"))
            (:Combo2.Branch
              (Class|SFABlogComboGameplayAbility|AddGameplayTags "(GameplayTags=((TagName=\"Ability.Begin.Combo3\")))"))))
        (:OnNotifyEnd
          (switch name _notifyname
            (:Combo2.Input
              (Class|SFABlogComboGameplayAbility|RemoveGameplayTags "(GameplayTags=((TagName=\"Ability.Ready.Combo3\")))"))
            (:Combo2.Branch
              (Class|SFABlogComboGameplayAbility|RemoveGameplayTags "(GameplayTags=((TagName=\"Ability.Begin.Combo3\")))"))))))))

(event Ability|EventOnEndAbility
  (params (bWasCancelled :type Boolean))
  (Class|SFABlogComboGameplayAbility|RemoveGameplayTags "(GameplayTags=((TagName=\"Ability.Begin.Combo3\"),(TagName=\"Ability.Ready.Combo3\")))"))