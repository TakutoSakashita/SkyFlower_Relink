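; BP_Laser is a fired laser beam actor that extends and travels along its forward vector, then destroys itself after its active time.
; LaunchLaser starts it; Tick grows the end point to the maximum length, then slides both ends forward, updating the beam emitter's source and target.
; While growing, it periodically spawns moving BP_SFA_LaserCollision actors at the Aggressor's location to act as collision.
; Its per-tick line trace result is unused.
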(event EventTick
  (params (DeltaSeconds :type Float%20%28single-precision%29))
  (bind _laser (Variables|Default|GetLaser))
  (if (Variables|Default|GetbIsLaunch)
    (switch int (Variables|Default|GetLaserState)
      (:0
        (Utilities|FlowControl|Sequence
          (:then_0
            ;[1 1 1] レーザー発射中
            (CallFunction|Launching (Transformation|GetActorForwardVector) DeltaSeconds)
            (Variables|Default|SetTimer_Laser (+ DeltaSeconds (Variables|Default|GetTimer_Laser)) :!label _label)
            ;[1 1 1] 処理時間が終了したか
            (if (>= (Variables|Default|GetTimer_Laser) (Variables|Default|GetActiveTime))
              (Variables|Default|SetbIsLaunch false)
              (Actor|DestroyActor)
              (else
                (Collision|LineTraceByChannel (Variables|Default|GetBeginPos) (Variables|Default|GetEndPos) "TraceTypeQuery1" false 0 "None")
                (Class|ParticleSystemComponent|SetBeamSourcePoint _laser 0 (Variables|Default|GetBeginPos))
                (Class|ParticleSystemComponent|SetBeamTargetPoint _laser 0 (Variables|Default|GetEndPos)))))
          (:then_1
            ;[1 1 1] spawn collision
            (bind _output_get (Variables|Default|SetSpawnCollisionTimer (- (Variables|Default|GetSpawnCollisionTimer) (Utilities|Time|GetWorldDeltaSeconds))))
            (if (< _output_get 0.0)
              (Variables|Default|SetSpawnCollisionTimer 0.1)
              (bind _returnvalue (Game|SpawnActorfromClass "/Game/BP/SFA_BP/BP_SFA_LaserCollision.BP_SFA_LaserCollision_C" (Math|Transform|MakeTransform (Transformation|GetActorLocation (Variables|Default|GetAggressor)) "0, 0, 0" "1.000000,1.000000,1.000000") "AlwaysSpawn" "MultiplyWithRoot" 0 0))
              (bind _output_get_2 (Variables|Default|SetLaserCollisionActor _returnvalue))
              (Utilities|IsValid _output_get_2
                (:Is%20Valid
                  (Class|SFALaserCollision|Initialize _output_get_2 (Variables|Default|GetAggressor) (Transformation|GetActorForwardVector) (* (Variables|Default|GetLaserSpeed) (Utilities|Time|GetWorldDeltaSeconds)) 1e+01 1e+01))
                (:Is%20Not%20Valid
                  (Development|PrintString "SPAWN LASER COLLISION FAILED" true false "(R=0.000000,G=1.000000,B=0.306662,A=1.000000)" 1.0)))))))
      (:1
        ;[1 1 1] レーザー発射終了
        (CallFunction|Launched (Transformation|GetActorForwardVector) DeltaSeconds)
        (goto _label)))))

(fn ConstructionScript)

(fn LaunchLaser
  (params (InBeginPos :type Vector%20%28by%20ref%29))
  (bind _output_get (Variables|Default|SetBeginPos InBeginPos))
  (Variables|Default|SetEndPos _output_get)
  (Variables|Default|SetbIsLaunch true))

(fn Launching
  (params (InVector :type Vector%20%28by%20ref%29) (InDeltaTime :type Float%20%28double-precision%29))
  (if (> (* (Variables|Default|GetTimer_Laser) (Variables|Default|GetLaserSpeed)) (Variables|Default|GetLaserLength))
    (Variables|Default|SetLaserState 1)
    (else
      (Variables|Default|SetEndPos (+ (Variables|Default|GetEndPos) (* InVector (* InDeltaTime (Variables|Default|GetLaserSpeed))))))))

(fn Launched
  (params (InVector :type Vector%20%28by%20ref%29) (InDeltaTime :type Float%20%28double-precision%29))
  (LocalVariables|SetDeltaVector (* InVector (* InDeltaTime (Variables|Default|GetLaserSpeed))))
  (Variables|Default|SetBeginPos (+ (LocalVariables|GetDeltaVector) (Variables|Default|GetBeginPos)))
  (Variables|Default|SetEndPos (+ (LocalVariables|GetDeltaVector) (Variables|Default|GetEndPos))))