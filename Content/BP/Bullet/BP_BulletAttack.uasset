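; Bullet attack spawner Blueprint that fires timed volleys of projectiles from its own location.
; RandAttack and SideAttack set the attack mode and reset the shot counter; Tick spawns through a Delay of attack time over bullet count.
; Random mode sprays randomly rotated bullets, with roughly one in ten being larger and aimed at the player.
; Side mode alternates homing bullets between the actor's right and left.
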(event Custom|RandAttack
  (params (AttackTime :type Float%20%28double-precision%29) (BulletNum :type Integer))
  (Variables|Default|SetAttackMode 1)
  (Variables|Default|SetCurrentBulletNum 0))

(event Custom|SideAttack
  (params (AttackTime :type Float%20%28double-precision%29) (BulletNum :type Integer))
  (Variables|Default|SetAttackMode 2)
  (Variables|Default|SetCurrentBulletNum 0))

(event EventBeginPlay)

(event Collision|EventActorBeginOverlap
  (params (OtherActor :type Actor%20Object%20Reference)))

(event EventTick
  (params (DeltaSeconds :type Float%20%28single-precision%29))
  (bind _returnvalue (Math|Random|RandomFloat))
  (bind _returnvalue_2 (* _returnvalue 3.6e+02))
  (switch int (Variables|Default|GetAttackMode)
    (:1
      (if (> (Variables|Default|GetCurrentBulletNum) (stale Custom|RandAttack BulletNum))
        (Variables|Default|SetAttackMode 0)
        (else
          (Utilities|FlowControl|Delay (/ (stale Custom|RandAttack AttackTime) (stale Custom|RandAttack BulletNum)))
          (if (== (/ (Math|Random|RandomInteger 100) 10) 0)
            (Game|SpawnActorfromClass "/Game/BP/Bullet/BP_ForwardBullet.BP_ForwardBullet_C" (Math|Transform|MakeTransform (Transformation|GetActorLocation) (Math|Rotator|FindLookatRotation (Transformation|GetActorLocation) (Transformation|GetActorLocation (Game|Player|GetPlayerPawn 0))) "10.000000,10.000000,10.000000") "Undefined" "MultiplyWithRoot" 0 0)
            (Math|Integer|IncrementInt (Variables|Default|GetCurrentBulletNum))
            (else
              (Game|SpawnActorfromClass "/Game/BP/Bullet/BP_ForwardBullet.BP_ForwardBullet_C" (Math|Transform|MakeTransform (Transformation|GetActorLocation) (Math|Rotator|MakeRotator _returnvalue_2 _returnvalue_2 _returnvalue_2) "3.000000,3.000000,3.000000") "Undefined" "MultiplyWithRoot" 0 0)
              (Math|Integer|IncrementInt (Variables|Default|GetCurrentBulletNum)))))))
    (:2
      (if (> (Variables|Default|GetCurrentBulletNum) (stale Custom|SideAttack BulletNum))
        (Variables|Default|SetAttackMode 0)
        (else
          (Utilities|FlowControl|Delay (/ (stale Custom|SideAttack AttackTime) (stale Custom|SideAttack BulletNum)))
          (bind _output_get (Variables|Default|SetbIsRight (Class|KismetMathLibrary|XORBoolean (Variables|Default|GetbIsRight) true)))
          (if _output_get
            (Game|SpawnActorfromClass "/Game/BP/Bullet/BP_HomingBullet.BP_HomingBullet_C" (Math|Transform|MakeTransform (Transformation|GetActorLocation) (Math|Conversions|RotationFromXVector (Transformation|GetActorRightVector)) "3.000000,3.000000,3.000000") "Undefined" "MultiplyWithRoot" 0 0)
            (else
              (Game|SpawnActorfromClass "/Game/BP/Bullet/BP_HomingBullet.BP_HomingBullet_C" (Math|Transform|MakeTransform (Transformation|GetActorLocation) (Math|Conversions|RotationFromXVector (* (Transformation|GetActorRightVector) "-1.000000,-1.000000,-1.000000")) "3.000000,3.000000,3.000000") "Undefined" "MultiplyWithRoot" 0 0)))
          (Math|Integer|IncrementInt (Variables|Default|GetCurrentBulletNum)))))))

(fn ConstructionScript)