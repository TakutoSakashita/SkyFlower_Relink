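; BP_ForwardBullet is a projectile actor that flies straight along its forward vector and destroys itself after ActiveTime.
; Tick moves it by MoveSpeed each frame without delta-time scaling or sweep, then feeds the Delay that leads to destruction.
; Its Sphere component's overlap with an SFA_Player only prints a "Hit" debug string, applying no damage and leaving the bullet alive.
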(event OnComponentBeginOverlap(Sphere)
  (params (OverlappedComponent :type Primitive%20Component%20Object%20Reference) (OtherActor :type Actor%20Object%20Reference) (OtherComp :type Primitive%20Component%20Object%20Reference) (OtherBodyIndex :type Integer) (bFromSweep :type Boolean) (SweepResult :type Hit%20Result%20Structure%20%28by%20ref%29))
  (Utilities|Casting|CastToSFA_Player OtherActor)
  (Development|PrintString "Hit" true true "(R=1.000000,G=0.088091,B=0.000000,A=1.000000)"))

(event EventBeginPlay)

(event Collision|EventActorBeginOverlap
  (params (OtherActor :type Actor%20Object%20Reference)))

(event EventTick
  (params (DeltaSeconds :type Float%20%28single-precision%29))
  (Transformation|SetActorLocation (+ (Transformation|GetActorLocation) (* (Transformation|GetActorForwardVector) (Variables|Default|GetMoveSpeed))) false false)
  (Utilities|FlowControl|Delay (Variables|Default|GetActiveTime))
  (Actor|DestroyActor))

(fn ConstructionScript)