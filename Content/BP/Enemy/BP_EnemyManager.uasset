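; BP_EnemyManager tracks the enemies in the level and reports whether all of them are defeated.
; On BeginPlay it fills EnemyList with every BP_EnemyBase actor in the world.
; AddEnemy and RemoveEnemy events update the list at runtime, and IsAllEnemiesDefeated returns true when it is empty.
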(event Custom|RemoveEnemy
  (params (InEnemy :type BP%20Enemy%20Base%20Object%20Reference))
  ;[1 1 1] Remove
  (Utilities|Array|RemoveItem (Variables|Default|GetEnemyList) InEnemy))

(event Custom|SetAllEnemies
  ;[1 1 1] Find All Enemies and Set
  (bind _outactors (Actor|GetAllActorsOfClass "/Game/BP/Enemy/BP_EnemyBase.BP_EnemyBase_C"))
  (Variables|Default|SetEnemyList _outactors))

(event Custom|AddEnemy
  (params (InEnemy :type BP%20Enemy%20Base%20Object%20Reference))
  ;[1 1 1] Pushback
  (Utilities|Array|Add (Variables|Default|GetEnemyList) InEnemy))

(event EventBeginPlay
  ;[1 1 1] Init
  (CallFunction|SetAllEnemies))

(fn ConstructionScript)

(fn IsAllEnemiesDefeated
  ;[1 1 1] Check AllEnemies Defeated
  (return (<= (Utilities|Array|Length (Variables|Default|GetEnemyList)) 0)))