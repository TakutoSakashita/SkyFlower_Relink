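; BP_Burst is a fire effect actor that damages the player when its Niagara system reports particle data.
; BeginPlay registers the actor as the Niagara export callback through the BP_CallBack variable.
; Each callback hits player 0 with fixed damage through TakeDamageBPMessage, crediting the owner, and spawns BP_Fire01 at the player, without reading the particle data.
; The delayed self-destroy nodes are disconnected and never run.
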(event EventBeginPlay
  ;[1 1 1] Collision Event SetUp
  (Class|NiagaraComponent|SetVariableObject (Variables|Default|GetNiagara) "BP_CallBack" self))

(event EventParticleData
  (params (Data :type Array%20of%20Basic%20Particle%20Data%20Structures) (NiagaraSystem :type Niagara%20System%20Object%20Reference) (SimulationPositionOffset :type Vector%20%28by%20ref%29 :default "0, 0, 0"))
  ;[1 1 1] Overlap
  (Class|BPIDamageable|TakeDamageBP(Message) (Game|GetPlayerCharacter 0) (Components|GetOwner) 1e+02)
  (Game|SpawnActorfromClass "/Game/Effects/FIre/BP_Fire01.BP_Fire01_C" (Transformation|GetActorTransform (Game|GetPlayerCharacter 0)) "Undefined" "MultiplyWithRoot" 0 0))

(fn ConstructionScript)