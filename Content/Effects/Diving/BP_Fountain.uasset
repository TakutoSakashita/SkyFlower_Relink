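; BP_Fountain is a timed fountain hazard among the Diving effects that damages the player on contact.
; After a short delay from BeginPlay, a timeline lerps the Box's relative height and Z scale to grow the hit volume, then the actor destroys itself after a pause.
; Overlap by BP_SFA_Player_modelTest sends fixed damage to player character 0 rather than the overlapping actor.
; Collision, Niagara lifetime and fire-spawn nodes are disconnected.
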(event OnComponentBeginOverlap(Box)
  (params (OverlappedComponent :type Primitive%20Component%20Object%20Reference) (OtherActor :type Actor%20Object%20Reference) (OtherComp :type Primitive%20Component%20Object%20Reference) (OtherBodyIndex :type Integer) (bFromSweep :type Boolean) (SweepResult :type Hit%20Result%20Structure%20%28by%20ref%29))
  ;[1 1 1] hit
  (Utilities|Casting|CastToBP_SFA_Player_modelTest OtherActor)
  (Development|PrintString "DivingHit")
  (Class|BPIDamageable|TakeDamageBP(Message) (Game|GetPlayerCharacter 0) (Components|GetOwner) 1e+02))

(event EventBeginPlay
  (Utilities|FlowControl|Delay 1.4)
  (bind _新規track_0 (Timeline|HeightTimeline Play)
    (:Update
      ;[1 1 1] begin
      (Utilities|FlowControl|Sequence
        (:then_0
          (Transformation|SetRelativeLocation (Variables|Default|GetBox) (Math|Vector|MakeVector 1.0 1.0 (Math|Float|Lerp 1.0 (Variables|Default|GetTargetLocationHeight) _新規track_0)) false false))
        (:then_1
          (Transformation|SetRelativeScale3D (Variables|Default|GetBox) (Math|Vector|MakeVector 1.0 1.0 (Math|Float|Lerp 1.0 (Variables|Default|GetTargetHeight) _新規track_0))))))
    (:Finished
      ;[1 1 1] end
      (Utilities|FlowControl|Delay 1.0)
      (Actor|DestroyActor))))

(fn ConstructionScript)