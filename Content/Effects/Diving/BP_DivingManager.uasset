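; Manager actor that spawns BP_Diving effect actors around the middle boss when OnDiving is called; nothing in its own live logic calls it.
; OnDiving validates a looked-up BP_MiddleBoss, but positions spawns from the BossMidlle variable, which is not assigned here.
; It places three raised spawns using the boss's forward and right vectors: far ahead, front-left and front-right, the last lacking a class.
; OnDestroy removes the manager.
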(event EventBeginPlay)

(event EventTick
  (params (DeltaSeconds :type Float%20%28single-precision%29)))

(fn ConstructionScript)

(fn OnDiving
  (bind _bossmidlle (Variables|Default|GetBossMidlle))
  (bind _bossmidlle_2 (Variables|Default|GetBossMidlle))
  (bind _bossmidlle_3 (Variables|Default|GetBossMidlle))
  (bind _returnvalue (Actor|GetActorOfClass "/Game/BP/SFA_BP/Boss/BP_MiddleBoss.BP_MiddleBoss_C"))
  (Utilities|IsValid _returnvalue
    (:Is%20Valid
      (Game|SpawnActorfromClass "/Game/Effects/Diving/BP_Diving.BP_Diving_C" (Math|Transform|MakeTransform (+ (* (Transformation|GetActorForwardVector _bossmidlle) (Math|Float|Absolute(Float) 2e+04)) (Transformation|GetActorLocation _bossmidlle) "0.000000,0.000000,1000.000000") (Transformation|GetActorRotation _bossmidlle)) "Undefined" "MultiplyWithRoot" 0 0)
      (Game|SpawnActorfromClass "/Game/Effects/Diving/BP_Diving.BP_Diving_C" (Math|Transform|MakeTransform (+ (* (Transformation|GetActorForwardVector _bossmidlle_2) (Math|Float|Absolute(Float) 1e+04)) (* (Transformation|GetActorRightVector _bossmidlle_2) "-13000.000000,-13000.000000,0.000000") (Transformation|GetActorLocation _bossmidlle_2) "0.000000,0.000000,1000.000000") (Transformation|GetActorRotation _bossmidlle_2)) "Undefined" "MultiplyWithRoot" 0 0)
      (Game|SpawnActorfromClass "/Game/Effects/Diving/BP_Diving.BP_Diving_C" (Math|Transform|MakeTransform (+ (* (Transformation|GetActorForwardVector _bossmidlle_3) (Math|Float|Absolute(Float) 1e+04)) (* (Transformation|GetActorRightVector _bossmidlle_3) (Math|Float|Absolute(Float) -1.3e+04)) (Transformation|GetActorLocation _bossmidlle_3) "0.000000,0.000000,1000.000000") (Transformation|GetActorRotation _bossmidlle_3)) "Undefined" "MultiplyWithRoot" 0 0))))

(fn OnDestroy
  (Actor|DestroyActor))