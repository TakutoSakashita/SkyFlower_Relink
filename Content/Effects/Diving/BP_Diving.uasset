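; BP_Diving is a diving effect actor that grows a Box component vertically over time.
; Two seconds after BeginPlay, a height timeline drives the Box's relative Z location and Z scale from 1 toward TargetLocationHeight and TargetHeight.
; Both lerps share the same timeline track, so the offset and stretch stay in sync, while X and Y are set to constants.
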(event EventBeginPlay
  (Utilities|FlowControl|Delay 2.0)
  (bind _新規track_0 (Timeline|HeightTimeline Play)
    (:Update
      (Utilities|FlowControl|Sequence
        (:then_0
          (Transformation|SetRelativeLocation (Variables|Default|GetBox) (Math|Vector|MakeVector 1.0 1.0 (Math|Float|Lerp 1.0 (Variables|Default|GetTargetLocationHeight) _新規track_0)) false false))
        (:then_1
          (Transformation|SetRelativeScale3D (Variables|Default|GetBox) (Math|Vector|MakeVector 1.0 1.0 (Math|Float|Lerp 1.0 (Variables|Default|GetTargetHeight) _新規track_0))))))))

(fn ConstructionScript)