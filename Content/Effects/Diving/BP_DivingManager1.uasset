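; BP_DivingManager1 is a manager actor that spawns BP_Fountain actors around the middle boss, apparently as diving effects.
; On BeginPlay it finds BP_MiddleBoss and spawns a fountain at a fixed world-space offset along X from the boss's location.
; Its OnDiving function repeats the lookup and spawns another fountain at a different X/Y offset; nothing in this Blueprint calls it.
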(event EventBeginPlay
  (bind _returnvalue (Actor|GetActorOfClass "/Game/BP/SFA_BP/Boss/BP_MiddleBoss.BP_MiddleBoss_C"))
  (Game|SpawnActorfromClass "/Game/Effects/Diving/BP_Fountain.BP_Fountain_C" (Math|Conversions|ToTransform(Vector) (+ (Transformation|GetActorLocation _returnvalue) "20000.000000,0.000000,0.000000")) "Undefined" "MultiplyWithRoot" 0 0))

(event Collision|EventActorBeginOverlap
  (params (OtherActor :type Actor%20Object%20Reference)))

(event EventTick
  (params (DeltaSeconds :type Float%20%28single-precision%29)))

(fn ConstructionScript)

(fn OnDiving
  (bind _returnvalue (Actor|GetActorOfClass "/Game/BP/SFA_BP/Boss/BP_MiddleBoss.BP_MiddleBoss_C"))
  (Game|SpawnActorfromClass "/Game/Effects/Diving/BP_Fountain.BP_Fountain_C" (Math|Conversions|ToTransform(Vector) (+ (Transformation|GetActorLocation _returnvalue) "10000.000000,-13000.000000,0.000000")) "Undefined" "MultiplyWithRoot" 0 0))